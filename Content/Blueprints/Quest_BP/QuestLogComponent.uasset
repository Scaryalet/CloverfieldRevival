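; Quest log component that tracks active and completed quest IDs and spawns a Quest_Base actor for each added quest.
; It answers active-quest queries and finds a quest's actor by searching the spawned list for a matching ID.
; Turn-in prints the current stage's XP reward, then moves the ID to completed, leaving the actor in the list.
; TrackQuest is an empty stub.
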(event EventBeginPlay)

(event EventTick
  (params (DeltaSeconds :type Float%20%28single-precision%29)))

(fn AddNewQuest
  (params (QuestID :type Name))
  (Utilities|Array|AddUnique (Variables|Default|GetCurrentActiveQuests) QuestID)
  (bind _returnvalue (Game|SpawnActorfromClass "/Game/Blueprints/Quest_BP/Quest_Base.Quest_Base_C" (Math|Transform|MakeTransform "0, 0, 0" "0, 0, 0" "1.000000,1.000000,1.000000") "Undefined" "MultiplyWithRoot" 0 QuestID 0))
  (Utilities|Array|Add (Variables|Default|GetCurrentQuests) _returnvalue))

(fn CompleteQuest
  (params (QuestID :type Name))
  (Utilities|Array|AddUnique (Variables|Default|GetCompletedQuests) QuestID)
  (Utilities|Array|RemoveItem (Variables|Default|GetCurrentActiveQuests) QuestID))

(fn QueryActiveQuest
  (params (QuestID :type Name))
  (return (Utilities|Array|ContainsItem (Variables|Default|GetCurrentActiveQuests) QuestID)))

(fn TrackQuest)

(fn GetQuestActor
  (params (QuestID :type Name))
  (for _array_element (Variables|Default|GetCurrentQuests)
    (if (== (Variables|/Game/Blueprints/Quest_BP/Quest_Base.Quest_Base_C|GetQuestID _array_element) QuestID)
      (return _array_element))))

(fn TurninQuest
  (params (QuestID :type Name))
  (Utilities|FlowControl|Sequence
    (:then_0
      (bind _array_element (CallFunction|GetQuestActor QuestID))
      (Development|PrintString (Utilities|String|ToString(Text) (Utilities|Text|FormatText "XP= {a}" (.XPReward (Utilities|Struct|BreakFStageDetails (Variables|/Game/Blueprints/Quest_BP/Quest_Base.Quest_Base_C|GetCurrentStageDetails _array_element)))))))
    (:then_1
      (CallFunction|CompleteQuest QuestID))))