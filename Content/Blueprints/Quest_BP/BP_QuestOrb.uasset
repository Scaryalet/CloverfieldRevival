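; Quest orb actor that shows an interact prompt and opens a quest UI when the player is nearby.
; BeginPlay creates both widgets, and Box overlaps toggle the prompt for any actor.
; Character overlap enables the orb's input, while ending it calls DisableInput on the player controller.
; F shows the quest UI; pressing E removes it and releasing E destroys the orb.
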(event OnComponentBeginOverlap(Box)
  (params (OverlappedComponent :type Primitive%20Component%20Object%20Reference) (OtherActor :type Actor%20Object%20Reference) (OtherComp :type Primitive%20Component%20Object%20Reference) (OtherBodyIndex :type Integer) (bFromSweep :type Boolean) (SweepResult :type Hit%20Result%20Structure%20%28by%20ref%29))
  (if true
    (UserInterface|Viewport|AddtoViewport (Variables|Default|GetInteractVar) 0)))

(event OnComponentEndOverlap(Box)
  (params (OverlappedComponent :type Primitive%20Component%20Object%20Reference) (OtherActor :type Actor%20Object%20Reference) (OtherComp :type Primitive%20Component%20Object%20Reference) (OtherBodyIndex :type Integer))
  (if true
    (Widget|RemovefromParent (Variables|Default|GetInteractVar))))

(event EventTick
  (params (DeltaSeconds :type Float%20%28single-precision%29)))

(event EventBeginPlay
  (Utilities|FlowControl|Sequence
    (:then_0
      (bind _returnvalue (UserInterface|CreateWidget "/Game/Blueprints/UI_BP/InteractButton.InteractButton_C"))
      (Variables|Default|SetInteractVar _returnvalue))
    (:then_1
      (bind _returnvalue_2 (UserInterface|CreateWidget "/Game/Blueprints/UI_BP/QuestUI.QuestUI_C"))
      (Variables|Default|SetQuestImages _returnvalue_2))))

(event Collision|EventActorBeginOverlap
  (params (OtherActor :type Actor%20Object%20Reference))
  (Utilities|Casting|CastToBP_ThirdPersonCharacter OtherActor)
  (Input|EnableInput (Game|GetPlayerController 0)))

(event Collision|EventActorEndOverlap
  (params (OtherActor :type Actor%20Object%20Reference))
  (Utilities|Casting|CastToBP_ThirdPersonCharacter OtherActor)
  (Input|DisableInput (Game|GetPlayerController 0) 0))

(event Input|KeyboardEvents|F
  (params (Key :type Key%20Structure :default "None"))
  (:Pressed
    (UserInterface|Viewport|AddtoViewport (Variables|Default|GetQuestImages) 0)))

(event Input|KeyboardEvents|E
  (params (Key :type Key%20Structure :default "None"))
  (:Pressed
    (Widget|RemovefromParent (Variables|Default|GetQuestImages)))
  (:Released
    (Actor|DestroyActor)))

(fn ConstructionScript)