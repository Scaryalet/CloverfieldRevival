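; SwordMaster is a quest-giver NPC that hands out a sword when interacted with.
; InteractWith forwards to the QuestGiverComponent, calls UpdateLevel, then runs GiveWeapons.
; GiveWeapons spawns an iron, steel or diamond sword at a small offset from the NPC according to NPCLevel, with no guard against repeat spawns.
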(event EventBeginPlay
  (|CallParentFunction) ; This node is disabled and will not be called.\nDrag off pins to build functionality.
)

(event Collision|EventActorBeginOverlap
  (params (OtherActor :type Actor%20Object%20Reference))
  (|CallParentFunction OtherActor) ; This node is disabled and will not be called.\nDrag off pins to build functionality.
)

(event EventTick
  (params (DeltaSeconds :type Float%20%28single-precision%29))
  (|CallParentFunction DeltaSeconds) ; This node is disabled and will not be called.\nDrag off pins to build functionality.
)

(fn ConstructionScript
  (|CallParentFunction))

(fn Interactwith
  (Default|Interactwith (Variables|Default|GetQuestGiverComponent))
  (CallFunction|UpdateLevel)
  (CallFunction|GiveWeapons)
  (return ""))

(fn GiveWeapons
  (if (== (Variables|Default|GetNPCLevel) 1.0)
    (Game|SpawnActorfromClass "/Game/Blueprints/Weapons/WeaponBP/IronSword.IronSword_C" (Math|Transform|MakeTransform (+ (Transformation|GetActorLocation) "15.000000,15.000000,5.000000") "0, 0, 0" "1.000000,1.000000,1.000000") "Undefined" "MultiplyWithRoot" 0 0)
    (elif (== (Variables|Default|GetNPCLevel) 2.0)
      (Game|SpawnActorfromClass "/Game/Blueprints/Weapons/WeaponBP/SteelSword.SteelSword_C" (Math|Transform|MakeTransform (+ (Transformation|GetActorLocation) "15.000000,15.000000,5.000000") "0, 0, 0" "1.000000,1.000000,1.000000") "Undefined" "MultiplyWithRoot" 0 0)
      (elif (== (Variables|Default|GetNPCLevel) 3.0)
        (Game|SpawnActorfromClass "/Game/Blueprints/Weapons/WeaponBP/DiamondSword.DiamondSword_C" (Math|Transform|MakeTransform (+ (Transformation|GetActorLocation) "15.000000,15.000000,5.000000") "0, 0, 0" "1.000000,1.000000,1.000000") "Undefined" "MultiplyWithRoot" 0 0)))))