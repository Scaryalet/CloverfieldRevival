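; Master NPC Blueprint that wanders near its house and tracks a level tied to quest progress.
; From BeginPlay, AI moves chain on success, roaming to random nearby reachable points and returning to HouseLocation after straying too far from HouseBP.
; UpdateLevel raises NPCLevel through three stages as the player completes the QuestGiverComponent's chained quests.
; InteractWith and GetSocketInfo are empty, leaving the quest interaction and UpdateLevel call disconnected.
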(event Custom|RandomRoam
  (AI|AIMoveTo self (.RandomLocation (AI|Navigation|GetRandomReachablePointinRadius (Transformation|GetActorLocation) 5e+02 0 0)) 0 5.0 false
    (:OnSuccess
      (if (>= (Transformation|GetHorizontalDistanceTo (Variables|Default|GetHouseBP)) 5e+02)
        (Variables|Default|SetShouldReturnHome true)
        (CallFunction|NextAction)
        (else
          (Variables|Default|SetShouldReturnHome false)
          (CallFunction|NextAction))))))

(event Custom|NextAction
  (if (Variables|Default|GetShouldReturnHome)
    (CallFunction|ReturnHome)
    (else
      (CallFunction|RandomRoam))))

(event Custom|ReturnHome
  (AI|AIMoveTo 0 (Variables|Default|GetHouseLocation) 0 5.0 false
    (:OnSuccess
      (Variables|Default|SetShouldReturnHome false)
      (CallFunction|NextAction))))

(event EventBeginPlay
  (CallFunction|NextAction))

(event Collision|EventActorBeginOverlap
  (params (OtherActor :type Actor%20Object%20Reference)))

(event EventTick
  (params (DeltaSeconds :type Float%20%28single-precision%29)))

(fn ConstructionScript)

(fn UpdateLevel
  (if (not (not (Default|QueryActiveQuest (Variables|/Game/Blueprints/PlayerCharacter/BP_ThirdPersonCharacter.BP_ThirdPersonCharacter_C|GetQuestLogComponent (CallFunction|GetMyPlayerCharacter)) (.rowname (Variables|/Game/Blueprints/Quest_BP/QuestGiverComponent.QuestGiverComponent_C|GetQuestData (Variables|Default|GetQuestGiverComponent))))))
    (bind _array_element (Default|GetQuestActor (Variables|/Game/Blueprints/PlayerCharacter/BP_ThirdPersonCharacter.BP_ThirdPersonCharacter_C|GetQuestLogComponent (CallFunction|GetMyPlayerCharacter)) (.rowname (Variables|/Game/Blueprints/Quest_BP/QuestGiverComponent.QuestGiverComponent_C|GetQuestData (Variables|Default|GetQuestGiverComponent)))))
    (if (Variables|/Game/Blueprints/Quest_BP/Quest_Base.Quest_Base_C|GetIsCompleted _array_element)
      (Variables|Default|SetNPCLevel 1.0)
      (if (not (not (Default|QueryActiveQuest (Variables|/Game/Blueprints/PlayerCharacter/BP_ThirdPersonCharacter.BP_ThirdPersonCharacter_C|GetQuestLogComponent (CallFunction|GetMyPlayerCharacter)) (.rowname (Variables|/Game/Blueprints/Quest_BP/QuestGiverComponent.QuestGiverComponent_C|GetQuestDataS2 (Variables|Default|GetQuestGiverComponent))))))
        (bind _array_element_2 (Default|GetQuestActor (Variables|/Game/Blueprints/PlayerCharacter/BP_ThirdPersonCharacter.BP_ThirdPersonCharacter_C|GetQuestLogComponent (CallFunction|GetMyPlayerCharacter)) (.rowname (Variables|/Game/Blueprints/Quest_BP/QuestGiverComponent.QuestGiverComponent_C|GetQuestDataS2 (Variables|Default|GetQuestGiverComponent)))))
        (if (Variables|/Game/Blueprints/Quest_BP/Quest_Base.Quest_Base_C|GetIsCompleted _array_element_2)
          (Variables|Default|SetNPCLevel 2.0)
          (if (not (not (Default|QueryActiveQuest (Variables|/Game/Blueprints/PlayerCharacter/BP_ThirdPersonCharacter.BP_ThirdPersonCharacter_C|GetQuestLogComponent (CallFunction|GetMyPlayerCharacter)) (.rowname (Variables|/Game/Blueprints/Quest_BP/QuestGiverComponent.QuestGiverComponent_C|GetQuestDataS3 (Variables|Default|GetQuestGiverComponent))))))
            (bind _array_element_3 (Default|GetQuestActor (Variables|/Game/Blueprints/PlayerCharacter/BP_ThirdPersonCharacter.BP_ThirdPersonCharacter_C|GetQuestLogComponent (CallFunction|GetMyPlayerCharacter)) (.rowname (Variables|/Game/Blueprints/Quest_BP/QuestGiverComponent.QuestGiverComponent_C|GetQuestDataS3 (Variables|Default|GetQuestGiverComponent)))))
            (if (Variables|/Game/Blueprints/Quest_BP/Quest_Base.Quest_Base_C|GetIsCompleted _array_element_3)
              (Variables|Default|SetNPCLevel 3.0))))))))

(fn GetSocketInfo
  (return 0))

(fn Interactwith)