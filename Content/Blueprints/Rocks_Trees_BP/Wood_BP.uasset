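; Wood_BP is an interactable wood pickup that returns "Wood" when interacted with and respawns through a controller.
; BeginPlay stores and prints its initial location.
; InteractWith passes its class and that location to the first ItemRespawnController found by GetAllActorsOfClass, then destroys the actor.
; Lookat and GetSocketInfo are empty stubs.
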(event EventBeginPlay
  (bind _output_get (Variables|Default|SetInitialLocation (Transformation|GetActorLocation)))
  (Development|PrintString (Utilities|String|ToString(Vector) _output_get)))

(event Collision|EventActorBeginOverlap
  (params (OtherActor :type Actor%20Object%20Reference)))

(event EventTick
  (params (DeltaSeconds :type Float%20%28single-precision%29)))

(event EventLookat)

(fn ConstructionScript)

(fn GetSocketInfo
  (return 0))

(fn Interactwith
  (bind _outactors (Actor|GetAllActorsOfClass "/Game/Blueprints/ItemRespawnController.ItemRespawnController_C"))
  (Default|RespawnItem (Utilities|Array|Get(acopy) _outactors) "Wood_BP_C" (Variables|Default|GetInitialLocation))
  (Actor|DestroyActor)
  (return "Wood"))