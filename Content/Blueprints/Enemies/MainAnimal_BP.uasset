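; MainAnimal_BP is an animal AI character that wanders, flees or attacks the player, playing ambient sounds at random intervals.
; DecideNextAction loops between slow short-range roaming and fast long-range fleeing, based on ShouldRun.
; Pawn sensing makes it chase a seen Player-tagged pawn and play an attack montage, whose notify runs a sphere trace to apply damage.
; Incoming damage only lowers Health, with no death handling here.
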(event OnSeePawn(PawnSensing)
  (params (Pawn :type Pawn%20Object%20Reference))
  (bind _returnvalue (Transformation|GetActorLocation))
  (if (Actor|ActorHasTag Pawn "Player")
    (Variables|/Script/Engine.CharacterMovementComponent|SetMaxWalkSpeed (Variables|Character|GetCharacterMovement) 4e+02)
    (AI|AIMoveTo self "0, 0, 0" (Game|GetPlayerCharacter 0) 1.8e+02 false
      (:OnSuccess
        (if (not (Variables|Default|GetIsAttacking))
          (Variables|Default|SetIsAttacking true)
          (Animation|Montage|PlayMontage (Variables|Character|GetMesh) (Variables|Default|GetAttackMontage)
            (:then
              (Audio|PlaySoundatLocation (Variables|Default|GetAttackSound) (Transformation|GetActorLocation) "0, 0, 0" 1.0 1.0 0.0 "/Game/Audio/SA_Animals.SA_Animals" 0 0 0))
            (:OnCompleted
              (Variables|Default|SetIsAttacking false))
            (:OnNotifyBegin
              (bind (_outhit _returnvalue_2) (Collision|SphereTraceForObjects _returnvalue (+ _returnvalue (* (Math|Vector|GetForwardVector (Transformation|GetActorRotation)) 2e+01)) 1.8e+02 (Utilities|Array|MakeArray "ObjectTypeQuery3") false 0 "ForDuration"))
              (if _returnvalue_2
                (Game|Damage|ApplyDamage (.HitActor (Collision|BreakHitResult _outhit)) (Variables|Default|GetAttackDamage) 0 0)
                (CallFunction|DecideNextAction false)))))))
    (else
      (CallFunction|DecideNextAction false))))

(event Custom|DecideNextAction
  (params (SkipDelay :type Boolean))
  (if SkipDelay
    _
    (else
      (Utilities|FlowControl|Delay (Math|Conversions|ToFloat(Integer) (Math|Random|RandomIntegerinRange 1 5)))))
  (if (Variables|Default|GetShouldRun)
    (CallFunction|RunAway)
    (else
      (CallFunction|RandomRoam))))

(event Custom|RandomRoam
  ;[1 1 1] Random Roam
  (Variables|/Script/Engine.CharacterMovementComponent|SetMaxWalkSpeed (Variables|Character|GetCharacterMovement) 1.5e+02)
  (AI|AIMoveTo self (.RandomLocation (AI|Navigation|GetRandomReachablePointinRadius (Transformation|GetActorLocation) 1.5e+03 0 0)) 0 5.0 false
    (:OnSuccess
      (CallFunction|DecideNextAction false))))

(event Custom|RunAway
  ;[1 1 1] Run Away
  (Variables|/Script/Engine.CharacterMovementComponent|SetMaxWalkSpeed (Variables|Character|GetCharacterMovement) 5e+02)
  (AI|AIMoveTo self (.RandomLocation (AI|Navigation|GetRandomReachablePointinRadius (Transformation|GetActorLocation) (Math|Random|RandomFloatinRange 1.5e+04 2.5e+04) 0 0)) 0 5.0 false
    (:OnSuccess
      (CallFunction|DecideNextAction true))))

(event EventBeginPlay
  (CallFunction|DecideNextAction false)
  (Utilities|FlowControl|Delay (Math|Random|RandomFloatinRange 3.0 15.0) :!label _label)
  (Audio|PlaySoundatLocation (Variables|Default|GetNormalSound) (Transformation|GetActorLocation) "0, 0, 0" 1.0 1.0 0.0 "/Game/Audio/SA_Animals.SA_Animals" 0 0 0)
  (goto _label))

(event Game|Damage|EventAnyDamage
  (params (Damage :type Float%20%28single-precision%29) (DamageType :type Damage%20Type%20Object%20Reference) (InstigatedBy :type Controller%20Object%20Reference) (DamageCauser :type Actor%20Object%20Reference))
  (Variables|Default|SetHealth (- (Variables|Default|GetHealth) Damage)))

(fn ConstructionScript)