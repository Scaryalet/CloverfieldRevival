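; HouseLVL0_BP is the level 0 house actor, which upgrades by replacing itself with HouseLVL1_BP.
; Its DestroyHouse event takes an NPC level and, when that equals one, spawns the next house at a hard-coded world location, stores and prints the level, then calls HouseDestroy to remove this actor.
; GetSocketInfo and InteractWith are empty stubs, and the construction script does nothing.
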(event Custom|HouseDestroy
  (Actor|DestroyActor))

(event EventBeginPlay)

(event Collision|EventActorBeginOverlap
  (params (OtherActor :type Actor%20Object%20Reference)))

(event EventTick
  (params (DeltaSeconds :type Float%20%28single-precision%29)))

(event EventDestroyHouse
  (params (NPCLVL :type Float%20%28double-precision%29))
  (if (== NPCLVL 1.0)
    (Game|SpawnActorfromClass "/Game/Blueprints/House_BP/HouseLVL1_BP.HouseLVL1_BP_C" (Math|Transform|MakeTransform "7703.000000,-8724.000000,-218.000000" "0, 0, 0" "1.000000,1.000000,1.000000") "Undefined" "MultiplyWithRoot" 0 0)
    (bind _output_get (Variables|Default|SetNPCLevel NPCLVL))
    (Development|PrintString (Utilities|String|ToString(Float) _output_get))
    (CallFunction|HouseDestroy)))

(fn ConstructionScript)

(fn GetSocketInfo
  (return 0))

(fn Interactwith
  (return ""))